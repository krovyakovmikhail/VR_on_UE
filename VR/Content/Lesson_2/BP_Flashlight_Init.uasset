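; BP_Flashlight_Init is a simple flashlight Blueprint that switches its SpotLight on and off with a button press.
; The ActionButtonAX input press drives a FlipFlop, whose alternating boolean sets the SpotLight's visibility without propagating to children.
; BeginPlay, overlap and Tick are disabled stubs, and the construction script only calls its parent.
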(event EventBeginPlay
  (|CallParentFunction) ; This node is disabled and will not be called.\nDrag off pins to build functionality.
)

(event Collision|EventActorBeginOverlap
  (params (OtherActor :type Actor%20Object%20Reference))
  (|CallParentFunction OtherActor) ; This node is disabled and will not be called.\nDrag off pins to build functionality.
)

(event EventTick
  (params (DeltaSeconds :type Float%20%28single-precision%29))
  (|CallParentFunction DeltaSeconds) ; This node is disabled and will not be called.\nDrag off pins to build functionality.
)

(event Input|ActionEvents|InputActionActionButtonAX
  (params (Key :type Key%20Structure))
  (:Pressed
    (bind _isa (Utilities|FlowControl|FlipFlop)
      (:A
        _)
      (:B
        _))
    (Rendering|SetVisibility (Variables|Default|GetSpotLight) _isa false)))

(fn ConstructionScript
  (|CallParentFunction))