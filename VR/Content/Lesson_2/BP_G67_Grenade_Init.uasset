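; Grenade Blueprint, named as a lesson asset, that prototypes a fuse countdown with debug text instead of an actual explosion.
; The TriggerReleased event passes through a DoOnce into a DoN limited by the Tick variable.
; When the counter equals Tick it prints "Bum"; otherwise it waits briefly and prints the remaining count.
; No loop back into the counter is present, and the default events are disabled.
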(event EventBeginPlay
  (|CallParentFunction) ; This node is disabled and will not be called.\nDrag off pins to build functionality.
)

(event Collision|EventActorBeginOverlap
  (params (OtherActor :type Actor%20Object%20Reference))
  (|CallParentFunction OtherActor) ; This node is disabled and will not be called.\nDrag off pins to build functionality.
)

(event EventTick
  (params (DeltaSeconds :type Float%20%28single-precision%29))
  (|CallParentFunction DeltaSeconds) ; This node is disabled and will not be called.\nDrag off pins to build functionality.
)

(event EventTriggerReleased
  (Utilities|FlowControl|DoOnce false
    (:Completed
      (bind _counter (Utilities|FlowControl|DoN (Variables|Default|GetTick))
        (:Exit
          (if (== _counter (Variables|Default|GetTick))
            (Development|PrintString "Bum")
            (else
              (Utilities|FlowControl|Delay 0.2)
              (Development|PrintString (Utilities|String|ToString(Integer) (- (Variables|Default|GetTick) _counter))))))))))

(fn ConstructionScript
  (|CallParentFunction))