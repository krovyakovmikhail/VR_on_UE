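; BP_SMG11_Init is an SMG11 weapon Blueprint that fires a projectile when its TriggerPressed event runs.
; The event spawns the Projectile class at the world location and rotation of an Arrow component, with the weapon as owner and the player pawn as instigator.
; BeginPlay, overlap and Tick are disabled stubs, and the construction script only calls its parent.
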(event EventBeginPlay
  (|CallParentFunction) ; This node is disabled and will not be called.\nDrag off pins to build functionality.
)

(event Collision|EventActorBeginOverlap
  (params (OtherActor :type Actor%20Object%20Reference))
  (|CallParentFunction OtherActor) ; This node is disabled and will not be called.\nDrag off pins to build functionality.
)

(event EventTick
  (params (DeltaSeconds :type Float%20%28single-precision%29))
  (|CallParentFunction DeltaSeconds) ; This node is disabled and will not be called.\nDrag off pins to build functionality.
)

(event EventTriggerPressed
  (bind _arrow (Variables|Default|GetArrow))
  (Game|SpawnActorfromClass "/Game/VRTemplate/Blueprints/Projectile.Projectile_C" (Math|Transform|MakeTransform (Transformation|GetWorldLocation _arrow) (Transformation|GetWorldRotation _arrow)) "Undefined" self (Game|Player|GetPlayerPawn 0)))

(fn ConstructionScript
  (|CallParentFunction))