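; BP_TRACE_SM_AR4 is a Blueprint, apparently an AR4 weapon from a lesson, that fires a line trace when its TriggerPressed event runs.
; The trace starts at component E and extends 10,000 units along its forward vector on the Visibility channel.
; Debug drawing is off and the hit result is unused, and the other events are disabled stubs.
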(event EventBeginPlay
  (|CallParentFunction) ; This node is disabled and will not be called.\nDrag off pins to build functionality.
)

(event Collision|EventActorBeginOverlap
  (params (OtherActor :type Actor%20Object%20Reference))
  (|CallParentFunction OtherActor) ; This node is disabled and will not be called.\nDrag off pins to build functionality.
)

(event EventTick
  (params (DeltaSeconds :type Float%20%28single-precision%29))
  (|CallParentFunction DeltaSeconds) ; This node is disabled and will not be called.\nDrag off pins to build functionality.
)

(event EventTriggerPressed
  (bind _e (Variables|Default|Gete))
  (bind _returnvalue (Transformation|GetWorldLocation _e))
  (Collision|LineTraceByChannel _returnvalue (+ _returnvalue (* (Math|Vector|GetForwardVector _e) 1e+04)) "TraceTypeQuery1" false 0 "None"))

(fn ConstructionScript
  (|CallParentFunction))